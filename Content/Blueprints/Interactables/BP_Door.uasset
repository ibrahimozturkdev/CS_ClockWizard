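; BP_Door is an interactable, replicated door that swings open and closed by rotating its Root in yaw.
; Interact toggles Opened only with authority, and is ignored while IsDoorAnimPlaying is set.
; The Opened RepNotify calls DoorInteraction, which plays the DoorAnimation timeline forward to open or in reverse to close, so the animation follows the replicated state.
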(event `/Game/Blueprints/Character/BPI_Interaction.Interact`
  (params (PlayerRef :type "/Game/Blueprints/Character/BP_PlayerBase Object Reference"))
  ;[0.1823 0.1823 0.1823] Interaction with Door
  (`/Engine/EditorBlueprintResources/ActorMacros.Switch Has Authority`
    (:`Authority`
      (if (not (`self.IsDoorAnimPlaying?`))
        (set `self.Opened?` (not (`self.Opened?`)))))))

(event `DoorInteraction`
  ;[0.2708 0.2708 0.2708] Door Interaction Animation
  (if (`self.Opened?`)
    (bind (_direction _z_vec) (`Timeline|DoorAnimation` :!via `PlayFromStart` :!label _label)
      (:`Update`
        (`SceneComponent.K2_SetRelativeRotation` (`self.Root`) (`KismetMathLibrary.MakeRotator` 0.0 0.0 _z_vec) false false)
        (set `self.IsDoorAnimPlaying?` true))
      (:`Finished`
        (set `self.IsDoorAnimPlaying?` false)))
    (else
      (goto _label :!via `ReverseFromEnd`))))

(fn `OnRep_Opened?`
  (`self.DoorInteraction`))

(fn `UserConstructionScript`
  (`parent.UserConstructionScript`))