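; BP_Tool_Stick is an interactable stick tool that players can pick up and equip, and that changes color on left click.
; Interact runs on the authority and sets the replicated ItemCollected flag if the player holds no tool; its OnRep has the player equip the stick.
; Left click sets a replicated random unit vector, whose OnRep writes it to the RandomColor material parameter on the mesh.
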(event `/Game/Blueprints/Character/BPI_Interaction.Interact`
  (params (PlayerRef :type "/Game/Blueprints/Character/BP_PlayerBase Object Reference"))
  ;[0.1979 0.1979 0.1979] Interaction
  (bind _output_get (set `self.Player Ref` PlayerRef))
  (`/Engine/EditorBlueprintResources/ActorMacros.Switch Has Authority`
    (:`Authority`
      (bind _isvalid (message `/Game/Blueprints/Character/BPI_PlayerCommunication.CheckCurrentHoldingTool` _output_get))
      (if (not _isvalid)
        (set `self.ItemCollected` true)))))

(event `/Game/Blueprints/Character/BPI_Interaction.LeftClick_Action`
  ;[1 0.4583 0.4583] Changing Color of Tool
  (set `self.RandomColor_Vec` (`KismetMathLibrary.RandomUnitVector`)))

(fn `OnRep_ItemCollected`
  (message `/Game/Blueprints/Character/BPI_PlayerCommunication.Equipt_Tool` (`self.Player Ref`) self))

(fn `OnRep_RandomColor_Vec`
  (`MeshComponent.SetVectorParameterValueOnMaterials` (`self.Mesh`) "RandomColor" (`self.RandomColor_Vec`)))

(fn `UserConstructionScript`
  (`parent.UserConstructionScript`))